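; World pickup item that registers with the player controller's inventory system while overlapped and has an interact widget showing name and quantity.
; On BeginPlay it derives an ID from its object name, destroys itself if the save marks it gone, and briefly hides until its quantity is set.
; The server saves removal state by ID in the GameInstance's save object, also storing transform, class and quantity for dropped items to respawn.
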(event `self.ReceiveBeginPlay`
  (bind _itemdatacomponent (`self.ItemDataComponent`))
  ;[0.09423 0.5411 1] load item
  (`self.ServerGetMyId`)
  (`self.Load Item`)
  ;[1 1 1] if you drop items, you must wait until the quantity is set
  (`self.SetActorHiddenInGame` true)
  (`KismetSystemLibrary.Delay` 0.2) ; wait until the item quantity is set
  (`self.SetActorHiddenInGame` false)
  (bind _aswbp_interact_message_with_details (cast `/Game/InventoryAndCraftingSystem/ItemChestInventory/UI/WBP_InteractMessageWithDetails` (`WidgetComponent.GetUserWidgetObject` (`self.Widget`))))
  (set `/Game/InventoryAndCraftingSystem/ItemChestInventory/UI/WBP_InteractMessageWithDetails.ItemName` (`KismetTextLibrary.Conv_NameToText` (`.RowName` (break `DataTableRowHandle` (`/Game/InventoryAndCraftingSystem/ItemChestInventory/Blueprints/AC_ItemDataComponent.ItemID` _itemdatacomponent)))) _aswbp_interact_message_with_details)
  (set `/Game/InventoryAndCraftingSystem/ItemChestInventory/UI/WBP_InteractMessageWithDetails.Quantity` (`/Game/InventoryAndCraftingSystem/ItemChestInventory/Blueprints/AC_ItemDataComponent.Quantity` _itemdatacomponent) _aswbp_interact_message_with_details)
  (`self.ServerSaveForRespawn` false))

(event `ServerSaveForRespawn`
  (params (NoLongerExist :type Boolean))
  (`self.Save Item For Respawn` NoLongerExist))

(event `serverSHOW`
  (params (MyPlayerController :type "/Game/InventoryAndCraftingSystem/ItemChestInventory/Blueprints/ControllerAndHUD/BP_MyPlayerController Object Reference"))
  ;[1 1 1] Show "interact" mesage (widget)
  (`/Game/InventoryAndCraftingSystem/ItemChestInventory/Blueprints/ControllerAndHUD/BP_MyPlayerController.ITEMShowMesage2` MyPlayerController self))

(event `ServerGetMyId`
  ;[0.09423 0.5411 1] CreateItemId
  (if (`KismetStringLibrary.IsEmpty` (`self.ItemID`))
    (set `self.ItemID` (`KismetSystemLibrary.GetObjectName` self))))

(event `serverHIDE`
  (params (MyPlayerController :type "/Game/InventoryAndCraftingSystem/ItemChestInventory/Blueprints/ControllerAndHUD/BP_MyPlayerController Object Reference"))
  ;[1 1 1] Show "interact" mesage (widget)
  (`/Game/InventoryAndCraftingSystem/ItemChestInventory/Blueprints/ControllerAndHUD/BP_MyPlayerController.ITEMHideMesage2` MyPlayerController self))

(event `ServerSave`
  (params (NoLongerExist :type Boolean))
  (`self.Save Item` NoLongerExist))

(event `self.Box.OnComponentBeginOverlap`
  (params (OverlappedComponent :type "PrimitiveComponent Object Reference") (OtherActor :type "Actor Object Reference") (OtherComp :type "PrimitiveComponent Object Reference") (OtherBodyIndex :type Integer) (bFromSweep :type Boolean) (SweepResult :type "HitResult Structure (by ref)"))
  ;[1 1 1] Collision Box
  (`self.ItemGOODToInteract` OtherActor))

(event `ShowMesage`
  ;[1 1 1] Show "interact" mesage (widget)
  (`SceneComponent.SetVisibility` (`self.Widget`) true false)
  (set `self.Enable Interaction?` true))

(event `self.Box.OnComponentEndOverlap`
  (params (OverlappedComponent :type "PrimitiveComponent Object Reference") (OtherActor :type "Actor Object Reference") (OtherComp :type "PrimitiveComponent Object Reference") (OtherBodyIndex :type Integer))
  ;[1 1 1] Collision Box
  (`self.ItemBADToInteract (remove from list)` OtherActor))

(event `HideMesage`
  ;[1 1 1] Show "interact" mesage (widget)
  (`SceneComponent.SetVisibility` (`self.Widget`) false false)
  (set `self.Enable Interaction?` false))

(fn `IsActive`
  (returns (`Enable Interaction?` :type Boolean))
  (return (`self.Enable Interaction?`)))

(fn `ItemBADToInteract (remove from list)`
  (params (PlayerCharacter :type "Actor Object Reference"))
  (bind _asbp_my_player_controller (cast `/Game/InventoryAndCraftingSystem/ItemChestInventory/Blueprints/ControllerAndHUD/BP_MyPlayerController` (`self.GetInstigatorController` PlayerCharacter)))
  (`/Game/InventoryAndCraftingSystem/ItemChestInventory/Blueprints/AC_Inventory_System.RemoveInteractiveActor` (`/Game/InventoryAndCraftingSystem/ItemChestInventory/Blueprints/ControllerAndHUD/BP_MyPlayerController.NEW_Inventory_System` _asbp_my_player_controller) self)
  (`self.serverHIDE` _asbp_my_player_controller))

(fn `ItemGOODToInteract`
  (params (PlayerCharacter :type "Actor Object Reference"))
  (bind _asbp_my_player_controller (cast `/Game/InventoryAndCraftingSystem/ItemChestInventory/Blueprints/ControllerAndHUD/BP_MyPlayerController` (`self.GetInstigatorController` PlayerCharacter)))
  (`/Game/InventoryAndCraftingSystem/ItemChestInventory/Blueprints/AC_Inventory_System.AddInteractiveActor` (`/Game/InventoryAndCraftingSystem/ItemChestInventory/Blueprints/ControllerAndHUD/BP_MyPlayerController.NEW_Inventory_System` _asbp_my_player_controller) self)
  (`self.serverSHOW` _asbp_my_player_controller))

(fn `Load Item`
  (bind _asmy_game_instance (cast `/Game/InventoryAndCraftingSystem/SavingAndLoading/MyGameInstance` (`GameplayStatics.GetGameInstance`)))
  (bind _as_bp_save_data (`/Game/InventoryAndCraftingSystem/SavingAndLoading/MyGameInstance.As BP Save Data` _asmy_game_instance))
  (if (and (`KismetSystemLibrary.IsServer`) (`/Game/InventoryAndCraftingSystem/SavingAndLoading/BP_SaveData.Load Used Items?` _as_bp_save_data))
    (bind (_value _returnvalue) (`BlueprintMapLibrary.Map_Find` (`/Game/InventoryAndCraftingSystem/SavingAndLoading/BP_SaveData.ItemNoLongerExist` _as_bp_save_data) (`self.ItemID`)))
    (if _returnvalue
      (if _value
        (`self.K2_DestroyActor`)))))

(fn `Save Item`
  (params (NoLongerExist :type Boolean :default true))
  (bind _itemid (`self.ItemID`))
  (bind _asmy_game_instance (cast `/Game/InventoryAndCraftingSystem/SavingAndLoading/MyGameInstance` (`GameplayStatics.GetGameInstance`)))
  (if (`KismetSystemLibrary.IsServer`)
    (bind _as_bp_save_data (`/Game/InventoryAndCraftingSystem/SavingAndLoading/MyGameInstance.As BP Save Data` _asmy_game_instance))
    (bind _itemnolongerexist (`/Game/InventoryAndCraftingSystem/SavingAndLoading/BP_SaveData.ItemNoLongerExist` _as_bp_save_data))
    (`BlueprintMapLibrary.Map_Add` _itemnolongerexist _itemid NoLongerExist)
    (if (`KismetStringLibrary.EqualEqual_StrStr` (`KismetSystemLibrary.GetDisplayName` self) (`self.ItemID`))
      (`self.Save Item For Respawn` true)
      (`BlueprintMapLibrary.Map_Remove` _itemnolongerexist _itemid))
    (`GameplayStatics.SaveGameToSlot` _as_bp_save_data (`/Game/InventoryAndCraftingSystem/SavingAndLoading/MyGameInstance.Slot Name` _asmy_game_instance))))

(fn `Save Item For Respawn`
  (params (NoLongerExist :type Boolean :default false))
  (bind _itemid (`self.ItemID`))
  (if (`/Game/InventoryAndCraftingSystem/ItemChestInventory/Blueprints/AC_ItemDataComponent.Dropped` (`self.ItemDataComponent`))
    (bind _asmy_game_instance (cast `/Game/InventoryAndCraftingSystem/SavingAndLoading/MyGameInstance` (`GameplayStatics.GetGameInstance`)))
    (if (`KismetSystemLibrary.IsServer`)
      (bind _as_bp_save_data (`/Game/InventoryAndCraftingSystem/SavingAndLoading/MyGameInstance.As BP Save Data` _asmy_game_instance))
      (`BlueprintMapLibrary.Map_Add` (`/Game/InventoryAndCraftingSystem/SavingAndLoading/BP_SaveData.ItemNoLongerExist` _as_bp_save_data) _itemid NoLongerExist)
      (`BlueprintMapLibrary.Map_Add` (`/Game/InventoryAndCraftingSystem/SavingAndLoading/BP_SaveData.Transform` _as_bp_save_data) _itemid (`self.GetTransform` self))
      (`BlueprintMapLibrary.Map_Add` (`/Game/InventoryAndCraftingSystem/SavingAndLoading/BP_SaveData.Class` _as_bp_save_data) _itemid (make `/Game/InventoryAndCraftingSystem/SavingAndLoading/F_DroppedItemsDetails` (`GameplayStatics.GetObjectClass` self) (make `/Game/InventoryAndCraftingSystem/ItemChestInventory/Blueprints/ItemsDataTable/F_SlotStruct` (`.RowName` (break `DataTableRowHandle` (`/Game/InventoryAndCraftingSystem/ItemChestInventory/Blueprints/AC_ItemDataComponent.ItemID` (`self.ItemDataComponent`)))) (`/Game/InventoryAndCraftingSystem/ItemChestInventory/Blueprints/AC_ItemDataComponent.Quantity` (`self.ItemDataComponent`)))))
      (if NoLongerExist
        (`BlueprintMapLibrary.Map_Remove` (`/Game/InventoryAndCraftingSystem/SavingAndLoading/BP_SaveData.ItemNoLongerExist` _as_bp_save_data) _itemid)
        (`BlueprintMapLibrary.Map_Remove` (`/Game/InventoryAndCraftingSystem/SavingAndLoading/BP_SaveData.Class` _as_bp_save_data) _itemid)
        (`BlueprintMapLibrary.Map_Remove` (`/Game/InventoryAndCraftingSystem/SavingAndLoading/BP_SaveData.Transform` _as_bp_save_data) _itemid))
      (`GameplayStatics.SaveGameToSlot` _as_bp_save_data (`/Game/InventoryAndCraftingSystem/SavingAndLoading/MyGameInstance.Slot Name` _asmy_game_instance)))))

(fn `UserConstructionScript`
  ;[1 0 0] Destroy actor if is default
  (if (== (`StaticMeshComponent.StaticMesh` (`self.StaticMesh`)) "/Game/InventoryAndCraftingSystem/ItemChestInventory/Meshes/SM_X.SM_X")
    (`ActorComponent.K2_DestroyComponent` (`self.Box`))))