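; Actor component that makes its owning item pickable, moving its ItemID and Quantity into a player or chest inventory.
; Interact adds to the player's inventory and refreshes it via MCUpdate, while AddItemtoChest targets a chest's inventory.
; On success it calls SaveItem on the BP_ItemDropped or BP_Item owner and destroys it.
; Failures raise full-inventory alerts, though the chest alert casts the owner to BP_MyPlayerController; BeginPlay enables owner replication.
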(event `self.ReceiveBeginPlay`
  (`Actor.SetReplicates` (`self.GetOwner`) true))

(event `/Game/InventoryAndCraftingSystem/ItemChestInventory/Blueprints/BI_IInteractInterface.Interact`
  (params (PlayerCharacter :type "/Game/InventoryAndCraftingSystem/ItemChestInventory/Blueprints/ControllerAndHUD/BP_MyPlayerController Object Reference"))
  (bind _returnvalue (`self.GetOwner`))
  (bind (_itemid_datatable _itemid_rowname) (break `DataTableRowHandle` (`self.ItemID`)))
  (bind _new_inventory_system (`/Game/InventoryAndCraftingSystem/ItemChestInventory/Blueprints/ControllerAndHUD/BP_MyPlayerController.NEW_Inventory_System` PlayerCharacter))
  (`/Engine/EditorBlueprintResources/StandardMacros.IsValid` _new_inventory_system
    (:`Is Valid`
      (bind _success (`/Game/InventoryAndCraftingSystem/ItemChestInventory/Blueprints/AC_Inventory_System.AddToInventory` _new_inventory_system _itemid_rowname (`self.Quantity`)))
      (`/Game/InventoryAndCraftingSystem/ItemChestInventory/Blueprints/AC_Inventory_System.MC_Update` _new_inventory_system)
      (if _success
        ;[0.09423 0.5411 1] save destroyed item
        (bind _asbp_item_dropped (cast `/Game/InventoryAndCraftingSystem/ItemChestInventory/Blueprints/Items/DroppedItems/BP_ItemDropped` _returnvalue)
          (:`then`
            (`/Game/InventoryAndCraftingSystem/ItemChestInventory/Blueprints/Items/DroppedItems/BP_ItemDropped.Save Item` _asbp_item_dropped true))
          (:`CastFailed`
            (bind _asbp_item (cast `/Game/InventoryAndCraftingSystem/ItemChestInventory/Blueprints/Items/NormalItems/BP_Item` _returnvalue))
            (`/Game/InventoryAndCraftingSystem/ItemChestInventory/Blueprints/Items/NormalItems/BP_Item.Save Item` _asbp_item true)))
        (`Actor.K2_DestroyActor` _returnvalue)
        (else
          (`/Game/InventoryAndCraftingSystem/ItemChestInventory/Blueprints/ControllerAndHUD/BP_MyPlayerController.Add ALERT` PlayerCharacter "Inventory is full"))))))

(event `/Game/InventoryAndCraftingSystem/ItemChestInventory/Blueprints/BI_IInteractInterface.AddItemToChest`
  (params (Chest :type "/Game/InventoryAndCraftingSystem/ItemChestInventory/Blueprints/Chests/Chest Object Reference"))
  (bind _returnvalue (`self.GetOwner`))
  (bind (_itemid_datatable _itemid_rowname) (break `DataTableRowHandle` (`self.ItemID`)))
  (bind _inventory_system (`/Game/InventoryAndCraftingSystem/ItemChestInventory/Blueprints/Chests/Chest.Inventory_System` Chest))
  (`/Engine/EditorBlueprintResources/StandardMacros.IsValid` _inventory_system
    (:`Is Valid`
      (bind _success (`/Game/InventoryAndCraftingSystem/ItemChestInventory/Blueprints/AC_Inventory_System.AddToInventory` _inventory_system _itemid_rowname (`self.Quantity`)))
      (if _success
        ;[0.09423 0.5411 1] save destroyed item
        (bind _asbp_item_dropped (cast `/Game/InventoryAndCraftingSystem/ItemChestInventory/Blueprints/Items/DroppedItems/BP_ItemDropped` _returnvalue)
          (:`then`
            (`/Game/InventoryAndCraftingSystem/ItemChestInventory/Blueprints/Items/DroppedItems/BP_ItemDropped.Save Item` _asbp_item_dropped true))
          (:`CastFailed`
            (bind _asbp_item (cast `/Game/InventoryAndCraftingSystem/ItemChestInventory/Blueprints/Items/NormalItems/BP_Item` _returnvalue))
            (`/Game/InventoryAndCraftingSystem/ItemChestInventory/Blueprints/Items/NormalItems/BP_Item.Save Item` _asbp_item true)))
        (`Actor.K2_DestroyActor` _returnvalue)
        (else
          (`/Game/InventoryAndCraftingSystem/ItemChestInventory/Blueprints/ControllerAndHUD/BP_MyPlayerController.Add ALERT` (cast `/Game/InventoryAndCraftingSystem/ItemChestInventory/Blueprints/ControllerAndHUD/BP_MyPlayerController` _returnvalue :!pure true) "Chest is full"))))))